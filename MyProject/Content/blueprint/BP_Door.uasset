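; BP_Door is a door actor that swings around its Hinge component when opened or closed.
; Open and Close only set a flag, which Tick polls to play or reverse RotationTimeline.
; The timeline's ZRot track lerps the Hinge's relative rotation from the actor rotation cached at BeginPlay to the same rotation with yaw replaced by ZTarget.
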(event EventBeginPlay
  (Variables|Default|SetStartingRotation (Transformation|GetActorRotation)))

(event EventTick
  (params (DeltaSeconds :type Float%20%28single-precision%29))
  (bind _startingrotation (Variables|Default|GetStartingRotation))
  (if (Variables|Default|GetShouldStartTimeline)
    (bind _zrot (Timeline|RotationTimeline Play)
      (:Update
        (Transformation|SetRelativeRotation (Variables|Default|Gethinge) (Math|Rotator|Lerp(Rotator) (Variables|Default|GetStartingRotation) (Math|Rotator|MakeRotator (.roll _startingrotation) (.pitch _startingrotation) (Variables|Default|GetZTarget)) _zrot) false false)))
    (else
      (Timeline|RotationTimeline Reverse))))

(fn ConstructionScript)

(fn Open
  (Variables|Default|SetShouldStartTimeline true))

(fn Close
  (Variables|Default|SetShouldStartTimeline false))