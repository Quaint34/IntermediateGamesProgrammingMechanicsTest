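; BP_Button is an overlap-triggered button actor that opens and closes a door in the level.
; When an actor begins overlapping, it turns its cube red and calls Open on a BP_Door; when the overlap ends, it restores the wall material and calls Close.
; The door is found on each event through GetActorOfClass on the ObjectToCast class variable, so it controls a single found instance.
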(event Collision|EventActorBeginOverlap
  (params (OtherActor :type Actor%20Object%20Reference))
  (Rendering|Material|SetMaterial (Variables|Default|GetCube) 0 "/Game/material/M_Red.M_Red")
  (bind _returnvalue (Actor|GetActorOfClass (Variables|Default|GetobjectToCast)))
  (bind _asbp_door (Utilities|Casting|CastToBP_Door _returnvalue))
  (Default|Open _asbp_door))

(event Collision|EventActorEndOverlap
  (params (OtherActor :type Actor%20Object%20Reference))
  (Rendering|Material|SetMaterial (Variables|Default|GetCube) 0 "/Game/StarterContent/Materials/M_Basic_Wall.M_Basic_Wall")
  (bind _returnvalue (Actor|GetActorOfClass (Variables|Default|GetobjectToCast)))
  (bind _asbp_door (Utilities|Casting|CastToBP_Door _returnvalue))
  (Default|Close _asbp_door))

(fn ConstructionScript)