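; BP_Cake is the goal object that triggers the win screen when its box is overlapped.
; A timeline, played from Tick, animates the Cake component's height and yaw by lerping between values from the starting and current actor transform, MoveLimit and RotLimit.
; Any overlap shows UW_Win, switches to UI-only input with a cursor and pauses the game.
; A name check for BP_FirstPersonCharacter is disconnected and never runs.
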(event OnComponentBeginOverlap(Box)
  (params (OverlappedComponent :type Primitive%20Component%20Object%20Reference) (OtherActor :type Actor%20Object%20Reference) (OtherComp :type Primitive%20Component%20Object%20Reference) (OtherBodyIndex :type Integer) (bFromSweep :type Boolean) (SweepResult :type Hit%20Result%20Structure%20%28by%20ref%29))
  (bind _returnvalue (Game|GetPlayerController 0))
  (bind _returnvalue_2 (UserInterface|CreateWidget "/Game/MainMenu/UW_Win.UW_Win_C"))
  (Variables|/Script/Engine.PlayerController|SetbShowMouseCursor _returnvalue true)
  (Input|SetInputModeUIOnly _returnvalue 0 "DoNotLock" false)
  (UserInterface|Viewport|AddtoViewport _returnvalue_2 0)
  (Game|SetGamePaused true))

(event EventTick
  (params (DeltaSeconds :type Float%20%28single-precision%29))
  (bind _returnvalue (Transformation|GetActorRotation))
  (bind _returnvalue_2 (Transformation|GetActorLocation))
  (bind (_direction _zmovement _zrotation) (Timeline|cake_anim Play)
    (:Update
      (Transformation|SetRelativeLocationAndRotation (Variables|Default|Getcake) (Math|Vector|Lerp(Vector) (Variables|Default|GetstartingLocation) (Math|Vector|MakeVector (.x _returnvalue_2) (.y _returnvalue_2) (+ (.z _returnvalue_2) (Variables|Default|GetmoveLimit))) _zmovement) (Math|Rotator|Lerp(Rotator) (Math|Rotator|MakeRotator (.roll _returnvalue) (.pitch _returnvalue) (Variables|Default|GetrotLimit)) (Variables|Default|GetstartingRotation) _zrotation) false false))))

(event EventBeginPlay
  (Variables|Default|SetstartingLocation (Transformation|GetActorLocation))
  (Variables|Default|SetstartingRotation (Transformation|GetActorRotation)))

(fn ConstructionScript)