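; BP_CollapsingRoof is a moving roof hazard that damages actors tagged Player when they overlap its Box.
; StartTimeline and StopTimeline set a flag that Tick polls to play or reverse MovementTimeline after separate start and end delays.
; The timeline lerps the Hinge's Z from the actor's starting location to ZLimit, applying that world-space start as a relative location.
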(event OnComponentBeginOverlap(Box)
  (params (OverlappedComponent :type Primitive%20Component%20Object%20Reference) (OtherActor :type Actor%20Object%20Reference) (OtherComp :type Primitive%20Component%20Object%20Reference) (OtherBodyIndex :type Integer) (bFromSweep :type Boolean) (SweepResult :type Hit%20Result%20Structure%20%28by%20ref%29))
  (if (Actor|ActorHasTag OtherActor "Player")
    (Game|Damage|ApplyDamage OtherActor 1.0 0 0)))

(event EventTick
  (params (DeltaSeconds :type Float%20%28single-precision%29))
  (bind _startinglocation (Variables|Default|GetstartingLocation))
  (if (Variables|Default|GetshouldStartTimeline)
    (Utilities|FlowControl|Delay (Variables|Default|GetstartDelay))
    (bind _platformz (Timeline|MovementTimeline Play)
      (:Update
        (Transformation|SetRelativeLocation (Variables|Default|Gethinge) (Math|Vector|Lerp(Vector) (Variables|Default|GetstartingLocation) (Math|Vector|MakeVector (.x _startinglocation) (.y _startinglocation) (Variables|Default|GetzLimit)) _platformz) false false)))
    (else
      (Utilities|FlowControl|Delay (Variables|Default|GetendDelay))
      (Timeline|MovementTimeline Reverse))))

(event EventBeginPlay
  (Variables|Default|SetstartingLocation (Transformation|GetActorLocation)))

(fn ConstructionScript)

(fn StartTimeline
  (Variables|Default|SetshouldStartTimeline true))

(fn StopTimeline
  (Variables|Default|SetshouldStartTimeline false))