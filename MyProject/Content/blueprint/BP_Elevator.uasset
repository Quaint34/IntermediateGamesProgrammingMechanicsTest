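; Elevator Blueprint that raises or lowers a Hinge component between its start position and a Z limit.
; StartTimeline and StopTimeline set a flag that Tick polls to play or reverse MovementTimeline after a start or end delay.
; While playing, the timeline interpolates the Hinge's relative location from the actor location cached at BeginPlay toward the same X and Y at ZLimit.
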(event EventTick
  (params (DeltaSeconds :type Float%20%28single-precision%29))
  (bind _startinglocation (Variables|Default|GetstartingLocation))
  (if (Variables|Default|GetshouldStartTimeline)
    (Utilities|FlowControl|Delay (Variables|Default|GetstartDelay))
    (bind _platformz (Timeline|MovementTimeline Play)
      (:Update
        (Transformation|SetRelativeLocation (Variables|Default|Gethinge) (Math|Vector|Lerp(Vector) (Variables|Default|GetstartingLocation) (Math|Vector|MakeVector (.x _startinglocation) (.y _startinglocation) (Variables|Default|GetzLimit)) _platformz) false false)))
    (else
      (Utilities|FlowControl|Delay (Variables|Default|GetendDelay))
      (Timeline|MovementTimeline Reverse))))

(event EventBeginPlay
  (Variables|Default|SetstartingLocation (Transformation|GetActorLocation)))

(fn ConstructionScript)

(fn StartTimeline
  (Variables|Default|SetshouldStartTimeline true))

(fn StopTimeline
  (Variables|Default|SetshouldStartTimeline false))