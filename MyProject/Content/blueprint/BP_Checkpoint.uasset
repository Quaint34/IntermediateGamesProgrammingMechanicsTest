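; BP_Checkpoint is a trigger actor that saves the player's progress when an actor tagged Player overlaps its Collision component.
; Each overlap creates a fresh BP_SaveData object, stores the checkpoint's own location and current level name, and asynchronously writes it to the BP_Game slot.
; The UW_Saving widget appears as the save starts and is removed after a fixed delay, independent of save completion.
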(event OnComponentBeginOverlap(Collision)
  (params (OverlappedComponent :type Primitive%20Component%20Object%20Reference) (OtherActor :type Actor%20Object%20Reference) (OtherComp :type Primitive%20Component%20Object%20Reference) (OtherBodyIndex :type Integer) (bFromSweep :type Boolean) (SweepResult :type Hit%20Result%20Structure%20%28by%20ref%29))
  (if (Actor|ActorHasTag OtherActor "Player")
    (bind _returnvalue (SaveGame|CreateSaveGameObject "/Game/blueprint/BP_SaveData.BP_SaveData_C"))
    (Variables|Default|SetSaveDataInstance _returnvalue)
    (Variables|/Game/blueprint/BP_SaveData.BP_SaveData_C|SetCheckpointLocation (Variables|Default|GetSaveDataInstance) (Transformation|GetActorLocation))
    (bind _returnvalue_2 (Game|GetCurrentLevelName true))
    (Variables|/Game/blueprint/BP_SaveData.BP_SaveData_C|SetCurrentPlayerLevel (Variables|Default|GetSaveDataInstance) _returnvalue_2)
    (|AsyncSaveGametoSlot (Variables|Default|GetSaveDataInstance) "BP_Game"
      (:then
        (bind _returnvalue_3 (UserInterface|CreateWidget "/Game/GUI/UW_Saving.UW_Saving_C"))
        (bind _output_get (Variables|Default|SetSaveWidget _returnvalue_3))
        (UserInterface|Viewport|AddtoViewport _output_get 0)
        (Utilities|FlowControl|Delay 2.0)
        (Widget|RemovefromParent (Variables|Default|GetsaveWidget))))))

(fn ConstructionScript)