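; Trap door actor that swings on a Hinge component when opened and swings back when closed.
; Open and Close only set a flag, which Tick polls every frame to play or reverse a timeline.
; The timeline drives a lerp of the hinge's relative rotation from the actor rotation cached at BeginPlay toward a target roll, keeping pitch and yaw.
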(event EventBeginPlay
  (Variables|Default|SetStartingRotation (Transformation|GetActorRotation)))

(event EventTick
  (params (DeltaSeconds :type Float%20%28single-precision%29))
  (bind _startingrotation (Variables|Default|GetStartingRotation))
  (if (Variables|Default|GetShouldStartTimeline)
    (bind _xrot (Timeline|MovementTimeline Play)
      (:Update
        (Transformation|SetRelativeRotation (Variables|Default|Gethinge) (Math|Rotator|Lerp(Rotator) (Variables|Default|GetStartingRotation) (Math|Rotator|MakeRotator (Variables|Default|GetXTarget) (.pitch _startingrotation) (.yaw _startingrotation)) _xrot) false false)))
    (else
      (Timeline|MovementTimeline Reverse))))

(fn ConstructionScript)

(fn Open
  (Variables|Default|SetShouldStartTimeline true))

(fn Close
  (Variables|Default|SetShouldStartTimeline false))